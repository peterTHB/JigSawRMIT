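; InteractableChair is a puzzle actor that shows an on-screen text component when something enters its sphere trigger.
; Sphere overlap begin and end toggle ShowingInstructions, which drives TextRender visibility, and enable or disable the actor's input for player controller 0.
; While input is enabled, pressing I sets the TextRender's content.
; Neither overlap event checks which actor triggered it.
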(event OnComponentBeginOverlap(Sphere)
  (params (OverlappedComponent :type Primitive%20Component%20Object%20Reference) (OtherActor :type Actor%20Object%20Reference) (OtherComp :type Primitive%20Component%20Object%20Reference) (OtherBodyIndex :type Integer) (bFromSweep :type Boolean) (SweepResult :type Hit%20Result%20Structure%20%28by%20ref%29))
  (Variables|Default|SetShowingInstructions true)
  (Input|EnableInput (Game|GetPlayerController 0))
  (Rendering|SetVisibility (Variables|Default|GetTextRender) (Variables|Default|GetShowingInstructions) false))

(event OnComponentEndOverlap(Sphere)
  (params (OverlappedComponent :type Primitive%20Component%20Object%20Reference) (OtherActor :type Actor%20Object%20Reference) (OtherComp :type Primitive%20Component%20Object%20Reference) (OtherBodyIndex :type Integer))
  (Variables|Default|SetShowingInstructions false)
  (Input|DisableInput (Game|GetPlayerController 0))
  (Rendering|SetVisibility (Variables|Default|GetTextRender) (Variables|Default|GetShowingInstructions) false))

(event EventBeginPlay)

(event Collision|EventActorBeginOverlap
  (params (OtherActor :type Actor%20Object%20Reference)))

(event EventTick
  (params (DeltaSeconds :type Float%20%28single-precision%29)))

(event Input|KeyboardEvents|I
  (params (Key :type Key%20Structure :default "None"))
  (:Pressed
    (Rendering|Components|TextRender|SetText (Variables|Default|GetTextRender) (Variables|Default|Gettext))))

(fn ConstructionScript)